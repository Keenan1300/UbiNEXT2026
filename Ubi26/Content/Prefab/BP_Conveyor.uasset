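; Conveyor actor that pushes actors overlapping MoveVolume, using an offset built from the Arrow's forward vector.
; Tick calls StartMove every frame, then offsets each overlap by forward plus (not times) delta-scaled Movespeed.
; Ispast makes the loop call Reset, snapping the conveyor to the Arrow's relative transform.
; Move/stop timers target "StopMoving" and "StartMoving", which mismatch the StopMove and StartMove events.
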(event Custom|StartMove
  (Variables|Default|SetIsmoving true)
  (Utilities|Time|SetTimerbyFunctionName 0 "StopMoving" (Variables|Default|GetMoveDuration)))

(event Custom|Reset
  (Transformation|SetActorTransform (Transformation|GetRelativeTransform (Variables|Default|GetArrow))))

(event Custom|StopMove
  (Variables|Default|SetIsmoving false)
  (Utilities|Time|SetTimerbyFunctionName 0 "StartMoving" (Variables|Default|GetStopDuration)))

(event Collision|EventActorBeginOverlap
  (params (OtherActor :type Actor%20Object%20Reference)))

(event EventTick
  (params (DeltaSeconds :type Float%20%28single-precision%29))
  (CallFunction|StartMove)
  (if (Variables|Default|GetIsmoving)
    (for _array_element (Collision|GetOverlappingActors (Variables|Default|GetMoveVolume) 0 :!class /Script/Engine.PrimitiveComponent)
      (Transformation|AddActorWorldOffset _array_element (+ (Math|Vector|GetForwardVector (Transformation|GetWorldRotation (Variables|Default|GetArrow))) (* DeltaSeconds (Variables|Default|Getmovespeed))))
      (if (Variables|Default|GetIspast)
        (CallFunction|Reset)
        (else
          (CallFunction|StartMove))))))

(event EventBeginPlay)

(fn ConstructionScript)