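; Barrel actor that can switch its mesh to a random material and destroy itself.
; SwapMaterial, also bound to Space, applies one of the first three MaterialChanger entries to BarrelMesh, and CE_Boom destroys the actor.
; A separate custom event caches the game mode.
; The EnableInput call and the construction script's dynamic-material setup are disconnected and never run.
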(event Custom|SwapMaterial
  (Rendering|Material|SetMaterial (Variables|Default|GetBarrelMesh) 0 (Utilities|Array|Get(acopy) (Variables|Default|GetMaterialChanger) (Math|Random|RandomIntegerinRange 0 2))))

(event Custom|CE_Boom
  (Actor|DestroyActor))

(event Custom|CustomEvent
  (bind _asgame_mode (Utilities|Casting|CastToGameMode (Game|GetGameMode)))
  (Variables|Default|SetAs%20Game%20Mode _asgame_mode))

(event Collision|EventActorBeginOverlap
  (params (OtherActor :type Actor%20Object%20Reference)))

(event EventTick
  (params (DeltaSeconds :type Float%20%28single-precision%29)))

(event EventBeginPlay)

(event Input|KeyboardEvents|SpaceBar
  (params (Key :type Key%20Structure :default "None"))
  (:Pressed
    (CallFunction|SwapMaterial)))

(fn ConstructionScript)